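; MainPlayer is a player-controlled Blueprint with camera-relative movement and an orbit-style camera.
; Move inputs follow the Gimbal's forward and right vectors, while look inputs yaw the Gimbal and pitch the SpringArm separately.
; Each Tick, the Body smoothly turns along the shortest path toward the movement input rotated into Gimbal space, holding its facing when input is idle.
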(event `self.ReceiveTick`
  (params (DeltaSeconds :type "Float (single-precision)"))
  (bind _body (`self.body`))
  (bind _returnvalue (`KismetMathLibrary.GreaterGreater_VectorRotator` (`KismetMathLibrary.MakeVector` (* (`self.GetInputAxisValue`) 100.0) (* (`self.GetInputAxisValue`) 100.0)) (`SceneComponent.K2_GetComponentRotation` (`self.Gimbal`))))
  (if (> (`KismetMathLibrary.VSize` _returnvalue) 0.1)
    (`SceneComponent.K2_SetWorldRotation` _body (`KismetMathLibrary.RLerp` (`SceneComponent.K2_GetComponentRotation` _body) (`KismetMathLibrary.Conv_VectorToRotator` _returnvalue) (* DeltaSeconds 5.0) true) false false)))

(event `InputAxis|MoveForward`
  (params (AxisValue :type "Float (single-precision)"))
  ;[1 1 1] Movement
  (`self.AddMovementInput` (`KismetMathLibrary.GetForwardVector` (`SceneComponent.RelativeRotation` (`self.Gimbal`))) AxisValue))

(event `InputAxis|MoveRight`
  (params (AxisValue :type "Float (single-precision)"))
  ;[1 1 1] Movement
  (`self.AddMovementInput` (`KismetMathLibrary.GetRightVector` (`SceneComponent.RelativeRotation` (`self.Gimbal`))) AxisValue))

(event `InputAxis|LookHorizontal`
  (params (AxisValue :type "Float (single-precision)"))
  ;[1 1 1] Camera Rotation
  (`SceneComponent.K2_AddLocalRotation` (`self.Gimbal`) (`KismetMathLibrary.Conv_VectorToRotator` (`KismetMathLibrary.CreateVectorFromYawPitch` AxisValue)) false false))

(event `InputAxis|LookVertical`
  (params (AxisValue :type "Float (single-precision)"))
  ;[1 1 1] Camera Rotation
  (`SceneComponent.K2_AddLocalRotation` (`self.SpringArm`) (`KismetMathLibrary.Conv_VectorToRotator` (`KismetMathLibrary.CreateVectorFromYawPitch` 0.0 AxisValue)) false false))

(fn `UserConstructionScript`)